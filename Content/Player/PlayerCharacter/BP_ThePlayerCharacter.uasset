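; Player character that manages oxygen and power reserves, interaction and object grabbing, with its HUD and button prompt widgets.
; A looping timer drains both resources, sprinting affects the drain rates, and the actor is destroyed when oxygen runs out.
; Interact sphere-traces and sends interface messages, while grab line-traces for IGrabbable actors and holds them with a timer-updated physics handle.
; Move and sprint input drive footstep audio through MasterAudio parameters.
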(event `ShowPrompt`
  ;[1 1 1] UI Prompt when Button Approached
  (`UserWidget.AddToViewport` (`self.ButtonPressUI`) 0))

(event `RemovePrompt`
  ;[1 1 1] UI Prompt when Button Approached
  (`Widget.RemoveFromParent` (`self.ButtonPressUI`)))

(event `self.ReceiveBeginPlay`
  (`|ExecutionSequence`
    (:`then_0`
      (set `self.currentOxygen` (`self.maxOxygen`))
      (set `self.currentPower` (`self.maxPower`))
      (set `self.originalOxygenDepletionRate` (`self.oxygenDepletionRate`)))
    (:`then_1`
      (bind _returnvalue (`|CreateWidget` "/Game/Tech/UI/PlayerUI/WBP_PlayerUI.WBP_PlayerUI_C" (`GameplayStatics.GetPlayerController` 0)))
      (bind _output_get (set `self.PlayerUI` _returnvalue))
      (`UserWidget.AddToViewport` _output_get 0)
      (bind _returnvalue_2 (`|CreateWidget` "/Game/Tech/UI/PlayerUI/WBP_ButtonPressUI.WBP_ButtonPressUI_C"))
      (set `self.ButtonPressUI` _returnvalue_2)
      (`KismetSystemLibrary.Delay` 0.2)
      (bind _outactors (`GameplayStatics.GetAllActorsOfClass` "/Game/Tech/Mech/BP_ProtoMech.BP_ProtoMech_C"))
      (set `self.MechRef` (`|GetArrayItem` _outactors)))
    (:`then_2`
      (`KismetSystemLibrary.K2_SetTimerDelegate` (delegate `CustomEvent`) 0.08 true))))

(event `CustomEvent`
  (bind (_currentpoweroutput _currentoxygenoutput) (`self.PowerUpdate`))
  (if (<= _currentoxygenoutput 0.0)
    (`self.K2_DestroyActor`)))

(event `EnhancedInput|/Game/Player/PlayerInput/PlayerInputActions/IA_Interact`
  (params (ActionValue :type Boolean) (ElapsedSeconds :type "Float (double-precision)") (TriggeredSeconds :type "Float (double-precision)") (InputAction :type "InputAction Object Reference" :default "/Game/Player/PlayerInput/PlayerInputActions/IA_Interact.IA_Interact"))
  (bind _returnvalue (`SceneComponent.K2_GetComponentLocation` (`self.InteractionLocation`)))
  ;[0 0 0] Interact
  (:`Started`
    (bind _outhit (`KismetSystemLibrary.SphereTraceSingle` _returnvalue _returnvalue 75.0 "TraceTypeQuery1"))
    (bind (_bblockinghit _binitialoverlap _time _distance _location _impactpoint _normal _impactnormal _physmat _hitactor) (`GameplayStatics.BreakHitResult` _outhit))
    (`/Engine/EditorBlueprintResources/StandardMacros.IsValid` _hitactor
      (:`Is Valid`
        (message `/Game/Tech/Mech/MechArmControls/BPI_CharacterToButton.LineTraceActivateButton` _hitactor (`self.MechRef`))
        (if (`KismetSystemLibrary.DoesImplementInterface` _hitactor "/Script/Collab2025.IInteractable")
          (message `IInteractable.Interact` _hitactor self))))))

(event `EnhancedInput|/Game/Player/PlayerInput/PlayerInputActions/IA_Sprint`
  (params (ActionValue :type Boolean) (ElapsedSeconds :type "Float (double-precision)") (TriggeredSeconds :type "Float (double-precision)") (InputAction :type "InputAction Object Reference" :default "/Game/Player/PlayerInput/PlayerInputActions/IA_Sprint.IA_Sprint"))
  (bind _footstepspeed (`self.footstepSpeed`))
  (bind _footstepaudio (`self.footstepAudio`))
  (:`Triggered`
    ;[1 1 1] Raises Audio Volume and Speed whilst sprinting
    (`self.Audio Parameter Setup` "speed" (/ _footstepspeed 1.35))
    (`self.Audio Parameter Setup` "volume" (* _footstepaudio 2.0))
    ;[1 1 1] DynamicOxygenDepletion
    (set `self.oxygenDepletionRate` (`self.sprintOxygenRate`)))
  (:`Completed`
    (`self.Audio Parameter Setup` "speed" _footstepspeed)
    (`self.Audio Parameter Setup` "volume" _footstepaudio)
    (set `self.oxygenDepletionRate` (`self.originalOxygenDepletionRate`))))

(event `EnhancedInput|/Game/Player/PlayerInput/PlayerInputActions/IA_Move`
  (params (ActionValue :type "Vector2D Structure") (ElapsedSeconds :type "Float (double-precision)") (TriggeredSeconds :type "Float (double-precision)") (InputAction :type "InputAction Object Reference" :default "/Game/Player/PlayerInput/PlayerInputActions/IA_Move.IA_Move"))
  (bind _masteraudio (`self.MasterAudio`))
  (:`Triggered`
    ;[1 1 1] Walking Sound Implementation
    (`/Engine/EditorBlueprintResources/StandardMacros.DoOnce` false :!label _label
      (:`Completed`
        (`AudioParameterControllerInterface.SetTriggerParameter` _masteraudio "Walk"))))
  (:`Completed`
    (`AudioParameterControllerInterface.SetTriggerParameter` _masteraudio "Stop")
    (goto _label :!via `Reset`)))

(event `/Game/Tech/Mech/EnergyConsole/BPI_PlayerToConsoleUI.E_DepleteResources`
  (params (oxygen :type "Float (double-precision)") (energy :type "Float (double-precision)"))
  ;[1 1 1] Depletes oxygen and energy
  (`|ExecutionSequence`
    (:`then_0`
      (set `self.currentOxygen` (- (`self.currentOxygen`) oxygen)))
    (:`then_1`
      (set `self.currentPower` (- (`self.currentPower`) energy)))))

(event `EnhancedInput|/Game/Player/PlayerInput/PlayerInputActions/IA_Grab`
  (params (ActionValue :type Boolean) (ElapsedSeconds :type "Float (double-precision)") (TriggeredSeconds :type "Float (double-precision)") (InputAction :type "InputAction Object Reference" :default "/Game/Player/PlayerInput/PlayerInputActions/IA_Grab.IA_Grab"))
  (bind __camera (`self._Camera`))
  (bind _returnvalue (`SceneComponent.K2_GetComponentLocation` __camera))
  ;[1 1 1] Grabs object and sets a timer whilst collided with a grabbable object
  (:`Started`
    (bind _outhit (`KismetSystemLibrary.LineTraceSingle` _returnvalue (+ _returnvalue (* (`SceneComponent.GetForwardVector` __camera) (`self.grabReach`))) "TraceTypeQuery1"))
    (bind (_bblockinghit _binitialoverlap _time _distance _location _impactpoint _normal _impactnormal _physmat _hitactor _hitcomponent) (`GameplayStatics.BreakHitResult` _outhit))
    (`/Engine/EditorBlueprintResources/StandardMacros.IsValid` _hitcomponent
      (:`Is Valid`
        (if (`KismetSystemLibrary.DoesImplementInterface` _hitactor "/Script/Collab2025.IGrabbable")
          (`PhysicsHandleComponent.GrabComponentAtLocationWithRotation` :`self` (`self.PhysicsHandle`) :`Component` _hitcomponent :`Location` (`SceneComponent.K2_GetComponentLocation` _hitcomponent))
          (bind _returnvalue_2 (`KismetSystemLibrary.K2_SetTimerDelegate` (delegate `KeepGrabbingItem`) 0.01 true))
          (set `self.grabTimer` _returnvalue_2)))))
  (:`Completed`
    (`KismetSystemLibrary.K2_ClearAndInvalidateTimerHandle` (`self.grabTimer`))
    (`PhysicsHandleComponent.ReleaseComponent` (`self.PhysicsHandle`))))

(event `KeepGrabbingItem`
  (bind __camera (`self._Camera`))
  ;[1 1 1] Grabs object and sets a timer whilst collided with a grabbable object
  (`PhysicsHandleComponent.SetTargetLocation` (`self.PhysicsHandle`) (+ (`SceneComponent.K2_GetComponentLocation` __camera) (* (`SceneComponent.GetForwardVector` __camera) (`self.grabReach`)))))

(fn `Audio Parameter Setup`
  (params (paramaterName :type Name) (float :type "Float (double-precision)"))
  (`AudioParameterControllerInterface.SetFloatParameter` (`self.MasterAudio`) paramaterName float))

(fn `CurrentResourceValues`
  (returns (oxygenOutput :type "Float (double-precision)") (energyOutput :type "Float (double-precision)"))
  (return (/ (`self.currentOxygen`) (`self.maxOxygen`)) (/ (`self.currentPower`) (`self.maxPower`))))

(fn `PowerUpdate`
  (returns (currentPowerOutput :type "Float (double-precision)") (currentOxygenOutput :type "Float (double-precision)"))
  (`|ExecutionSequence`
    (:`then_0`
      (set `self.currentOxygen` (- (`self.currentOxygen`) (`self.oxygenDepletionRate`)))
      (if (`self.bIsSprinting`)
        (set `self.currentPower` (- (`self.currentPower`) (* (`self.energyDepletionRate`) (`self._SprintBaseSpeedRatio`) (`self.PowerSprintMult`))))
        (else
          (set `self.currentPower` (- (`self.currentPower`) (`self.energyDepletionRate`))))))
    (:`then_1`
      (return (`self.currentPower`) (`self.currentOxygen`)))))

(fn `Pressing Button`
  (params (Range :type "Float (double-precision)"))
  (returns (Button :type "PrimitiveComponent Object Reference"))
  (bind _returnvalue (`GameplayStatics.GetPlayerCameraManager` 0))
  (bind _returnvalue_2 (`PlayerCameraManager.GetCameraLocation` _returnvalue))
  (bind _outhit (`KismetSystemLibrary.LineTraceSingle` _returnvalue_2 (+ _returnvalue_2 (* (`KismetMathLibrary.GetForwardVector` (`SceneComponent.K2_GetComponentRotation` (`PlayerCameraManager.TransformComponent` _returnvalue))) Range)) "TraceTypeQuery1" true))
  (if (`GameplayStatics.BreakHitResult` _outhit)
    (if (`ActorComponent.ComponentHasTag` (`.HitComponent` (`GameplayStatics.BreakHitResult` _outhit)) "Button")
      (set `self.ButtonPressed` true)
      (`GameplayStatics.PlaySound2D` "/Game/Tech/Mech/S_ButtonPress.S_ButtonPress" 1.0 1.0 0.0 null null)
      (else
        (set `self.ButtonPressed` false :!label _label)))
    (else
      (goto _label)))
  (return (`.HitComponent` (`GameplayStatics.BreakHitResult` _outhit))))

(fn `UserConstructionScript`)