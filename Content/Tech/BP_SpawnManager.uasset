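; BP_SpawnManager runs an enemy wave, spawning BP_TestEnemy actors and flagging when all of them are defeated.
; SpawnEnemies starts a looping timer that spawns one enemy at a time within a long, thin box around the given position.
; At the target count, a faster polling timer takes over, comparing defeated to spawned counts, then sets EnemiesCleared and resets both.
; The defeated count is not incremented within this Blueprint.
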(event `Check Defeated`
  (if (== (`self.EnemiesDefeated`) (`self.EnemiesSpawned`))
    (set `self.Enemies Cleared` true)
    (set `self.EnemiesSpawned` 0)
    (set `self.EnemiesDefeated` 0)
    (`KismetSystemLibrary.K2_ClearAndInvalidateTimerHandle` (stale `Spawning` _returnvalue))))

(event `Spawning`
  (if (>= (`self.EnemiesSpawned`) (`self.EnemiesToSpawn`))
    (`KismetSystemLibrary.K2_ClearAndInvalidateTimerHandle` (stale `Spawn Enemies` _returnvalue))
    (bind _returnvalue (`KismetSystemLibrary.K2_SetTimerDelegate` (delegate `Check Defeated`) 0.1 true))
    (else
      (`|SpawnActorFromClass` "/Game/Tech/BP_TestEnemy.BP_TestEnemy_C" (`KismetMathLibrary.MakeTransform` (`KismetMathLibrary.RandomPointInBoundingBox` (stale `Spawn Enemies` `Spawn Position`) (3000.0 50.0 0.0))) "AdjustIfPossibleButAlwaysSpawn" "MultiplyWithRoot" null null)
      (set `self.EnemiesSpawned` (+ (`self.EnemiesSpawned`) 1)))))

(event `Spawn Enemies`
  (params (`Spawn Position` :type "Vector Structure"))
  (set `self.Enemies Cleared` false)
  (bind _returnvalue (`KismetSystemLibrary.K2_SetTimerDelegate` (delegate `Spawning`) 3.0 true)))

(fn `UserConstructionScript`)