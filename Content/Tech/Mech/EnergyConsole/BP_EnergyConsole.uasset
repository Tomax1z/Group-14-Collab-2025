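; Mech energy console that shows oxygen and energy levels on a WBP_MechResource widget.
; On BeginPlay it caches the widget and starts a looping timer.
; Each timer tick queries the player pawn through the CurrentResourceValues interface message and sets both progress bars from the returned values.
; The console's own CurrentResourceValues function is a stub returning zeros.
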(event `self.ReceiveBeginPlay`
  ;[1 1 1] I can't think of any other way to do this...
  (bind _aswbp_mech_resource (cast `/Game/Tech/UI/MechUI/WBP_MechResource` (`WidgetComponent.GetWidget` (`self.Widget`))))
  (set `self.UI` _aswbp_mech_resource)
  (`KismetSystemLibrary.K2_SetTimerDelegate` (delegate `UpdateBars`) 0.1 true))

(event `UpdateBars`
  (bind _ui (`self.UI`))
  (bind (_oxygenoutput _energyoutput) (message `/Game/Tech/Mech/EnergyConsole/BPI_PlayerToConsoleUI.CurrentResourceValues` (`GameplayStatics.GetPlayerPawn` 0)))
  (`ProgressBar.SetPercent` (`/Game/Tech/UI/MechUI/WBP_MechResource.oxygenBar` _ui) _oxygenoutput)
  (`ProgressBar.SetPercent` (`/Game/Tech/UI/MechUI/WBP_MechResource.energyBar` _ui) _energyoutput))

(fn `CurrentResourceValues`
  (returns (oxygenOutput :type "Float (double-precision)") (energyOutput :type "Float (double-precision)"))
  (return 0.0 0.0))

(fn `UserConstructionScript`)