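; BP_ResourceConsole is a console that raises the player's oxygen or energy when a matching item touches its box.
; On overlap, it switches on ResourceType, checks for the oxygen tank or energy cell interface, calls IncreaseResources and destroys the item.
; IncreaseResources reuses the player pawn's EDepleteResourcesMessage to add resources, passing both amounts through a unary operation.
; Both of its Sequence branches lead into that same message call.
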(event `self.Box.OnComponentBeginOverlap`
  (params (OverlappedComponent :type "PrimitiveComponent Object Reference") (OtherActor :type "Actor Object Reference") (OtherComp :type "PrimitiveComponent Object Reference") (OtherBodyIndex :type Integer) (bFromSweep :type Boolean) (SweepResult :type "HitResult Structure (by ref)"))
  ;[1 1 1] Check to find what material it is. Then increase the value
  (switch `/Game/Tech/Mech/ResourceConsoles/E_Resources` (`self.resourceType`)
    (:`NewEnumerator0`
      (if (`KismetSystemLibrary.DoesImplementInterface` OtherActor "/Game/Tech/Mech/ResourceConsoles/BPI_OxygenTank.BPI_OxygenTank_C")
        (`self.IncreaseResources` (`self.valueIncrease`))
        (`self.K2_DestroyActor` OtherActor :!label _label)))
    (:`NewEnumerator1`
      (if (`KismetSystemLibrary.DoesImplementInterface` OtherActor "/Game/Tech/Mech/ResourceConsoles/BPI_EnergyCell.BPI_EnergyCell_C")
        (`self.IncreaseResources` 0.0 (`self.valueIncrease`))
        (goto _label)))))

(event `IncreaseResources`
  (params (oxygenValue :type "Float (double-precision)") (energyValue :type "Float (double-precision)"))
  ;[1 1 1] This allows you to actually increase values
  (`|ExecutionSequence`
    (:`then_0`
      (bind _result (`/Engine/EditorBlueprintResources/StandardMacros.NegateFloat` oxygenValue)
        (:`  `
          _)))
    (:`then_1`
      (bind _result_2 (`/Engine/EditorBlueprintResources/StandardMacros.NegateFloat` energyValue)
        (:`  `
          _))))
  (message `/Game/Tech/Mech/EnergyConsole/BPI_PlayerToConsoleUI.E_DepleteResources` (`GameplayStatics.GetPlayerPawn` 0) _result _result_2))

(fn `UserConstructionScript`)