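; Prototype mech actor with health, a cooldown-gated repair, and left and right arm actors found in the level at BeginPlay.
; Arm events forward rotate, swipe and grab calls, while a looping timer zeroes MoveSpeed when the player pawn's energy output runs out.
; Damage flashes tagged level point lights red or, at zero health, pauses into a death screen.
; Collider overlaps toggle the player character's button prompt.
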(event `Event Power Down`
  (set `self._MoveSpeed` 0.0))

(event `CheckForPower`
  (bind (_oxygenoutput _energyoutput) (message `/Game/Tech/Mech/EnergyConsole/BPI_PlayerToConsoleUI.CurrentResourceValues` (`GameplayStatics.GetPlayerPawn` 0)))
  (if (<= _energyoutput 0.0)
    (set `self._MoveSpeed` 0.0)))

(event `/Game/Tech/Mech/MechArmControls/BPI_ButtonToMech.ActivateRepair`
  (bind _health (`self.Health`))
  (bind _maxhealth (`self.MaxHealth`))
  ;[1 1 1] Repair
  (if (`self.CanRepair`)
    (set `self.CanRepair` false)
    (if (< _health _maxhealth)
      (set `self.Health` (`KismetMathLibrary.FClamp` (+ _health (`self.RepairAmount`)) 0.0 _maxhealth))
      (`KismetSystemLibrary.Delay` (`self.RepairCooldown`))
      (set `self.CanRepair` true))))

(event `self.ReceiveBeginPlay`
  ;[1 1 1] Not Good
  (`|ExecutionSequence`
    (:`then_0`
      (`KismetSystemLibrary.K2_SetTimerDelegate` (delegate `CheckForPower`) 0.1 true))
    (:`then_1`
      (bind _outactors (`GameplayStatics.GetAllActorsOfClass` "/Game/Tech/Mech/MechArms/BP_RightArm.BP_RightArm_C"))
      (set `self.RightArm` (`|GetArrayItem` _outactors))
      (bind _outactors_2 (`GameplayStatics.GetAllActorsOfClass` "/Game/Tech/Mech/MechArms/BP_LeftArm.BP_LeftArm_C"))
      (set `self.LeftArm` (`|GetArrayItem` _outactors_2))
      (set `self.Health` (`self.MaxHealth`)))))

(event `/Game/Tech/Mech/MechArmControls/BPI_ButtonToMech.MoveArmLeft`
  (params (`IsLeftSide?` :type Boolean))
  (if `IsLeftSide?`
    (`/Game/Tech/Mech/MechArms/BP_LeftArm.RotateArmLeft` (`self.LeftArm`))
    (else
      (`/Game/Tech/Mech/MechArms/BP_RightArm.RotateArmLeft` (`self.RightArm`)))))

(event `/Game/Tech/Mech/MechArmControls/BPI_ButtonToMech.ActivateSwipe`
  (params (`isLeft?` :type Boolean))
  ;[1 1 1] Swipe and Grab
  (if `isLeft?`
    (message `/Game/Tech/Mech/MechArmControls/BPI_ButtonToArm.ActivateSwipe` (`self.LeftArm`) true)
    (else
      (message `/Game/Tech/Mech/MechArmControls/BPI_ButtonToArm.ActivateSwipe` (`self.RightArm`) false))))

(event `/Game/Tech/Mech/MechArmControls/BPI_ButtonToMech.MoveArmRight`
  (params (`IsLeftSide?` :type Boolean))
  (if `IsLeftSide?`
    (`/Game/Tech/Mech/MechArms/BP_LeftArm.RotateArmRight` (`self.LeftArm`)))
  (`/Game/Tech/Mech/MechArms/BP_RightArm.RotateArmRight` (`self.RightArm`)))

(event `/Game/Tech/Mech/MechArmControls/BPI_ButtonToMech.ActivateArm`
  (params (`isLeft?` :type Boolean))
  ;[1 1 1] Swipe and Grab
  (if `isLeft?`
    (message `/Game/Tech/Mech/MechArmControls/BPI_ButtonToArm.ActivateGrab` (`self.LeftArm`))
    (else
      (message `/Game/Tech/Mech/MechArmControls/BPI_ButtonToArm.ActivateGrab` (`self.RightArm`)))))

(event `self.ReceiveAnyDamage`
  (params (Damage :type "Float (single-precision)") (DamageType :type "DamageType Object Reference") (InstigatedBy :type "Controller Object Reference") (DamageCauser :type "Actor Object Reference"))
  ;[0 0 0] Temp Health
  (bind _output_get (set `self.Health` (- (`self.Health`) Damage)))
  (if (<= _output_get 0.0)
    (`GameplayStatics.SetGamePaused` true)
    (set `PlayerController.bShowMouseCursor` true (`GameplayStatics.GetPlayerController` 0))
    (bind _returnvalue (`|CreateWidget` "/Game/Tech/UI/ScreenUI/WBP_DeathScreen.WBP_DeathScreen_C" (`GameplayStatics.GetPlayerController` 0)))
    (`UserWidget.AddToViewport` _returnvalue 0)
    (else
      (`self.Flash Lights`))))

(event `Flash Lights`
  ;[1 1 1] Flash all point lights with the tag "Mech Light" red, not sure how to get reference to level actors attached to mech otherwise, uses a float array to track their original intensity as some lights have different intensity values than others
  (bind _outactors (`GameplayStatics.GetAllActorsOfClassWithTag` "/Script/Engine.PointLight" "Mech Light"))
  (for _array_element _outactors
    (bind _lightcomponent (`Light.LightComponent` _array_element))
    (`LightComponent.SetLightColor` _lightcomponent (struct :`R` 0.776042 :`B` 0.058004 :`A` 1.0) true)
    (`KismetArrayLibrary.Array_Add` (`self.LightIntensities`) (`LightComponentBase.Intensity` _lightcomponent))
    (`LightComponent.SetIntensity` _lightcomponent 2000.0))
  (`KismetSystemLibrary.Delay` 1.0)
  (for (_array_element_2 _array_index) _outactors
    (bind _lightcomponent_2 (`Light.LightComponent` _array_element_2))
    (`LightComponent.SetLightColor` _lightcomponent_2 (struct :`R` 0.776042 :`G` 0.776042 :`B` 0.776042 :`A` 1.0) true)
    (`LightComponent.SetIntensity` _lightcomponent_2 (`|GetArrayItem` (`self.LightIntensities`) _array_index))))

(event `self.ButtonUICollider.OnComponentBeginOverlap`
  (params (OverlappedComponent :type "PrimitiveComponent Object Reference") (OtherActor :type "Actor Object Reference") (OtherComp :type "PrimitiveComponent Object Reference") (OtherBodyIndex :type Integer) (bFromSweep :type Boolean) (SweepResult :type "HitResult Structure (by ref)"))
  ;[1 1 1] UI Button Prompt
  (`self.ShowPromptToPlayer` OtherActor))

(event `ShowPromptToPlayer`
  (params (`Player Reference` :type "Actor Object Reference"))
  ;[1 1 1] UI Button Prompt
  (bind _asbp_the_player_character (cast `/Game/Player/PlayerCharacter/BP_ThePlayerCharacter` `Player Reference`))
  (`/Game/Player/PlayerCharacter/BP_ThePlayerCharacter.ShowPrompt` _asbp_the_player_character))

(event `RemovePromptToPlayer`
  (params (`Player Reference` :type "Actor Object Reference"))
  ;[1 1 1] UI Button Prompt
  (bind _asbp_the_player_character (cast `/Game/Player/PlayerCharacter/BP_ThePlayerCharacter` `Player Reference`))
  (`/Game/Player/PlayerCharacter/BP_ThePlayerCharacter.RemovePrompt` _asbp_the_player_character))

(event `self.ButtonUICollider1.OnComponentBeginOverlap`
  (params (OverlappedComponent :type "PrimitiveComponent Object Reference") (OtherActor :type "Actor Object Reference") (OtherComp :type "PrimitiveComponent Object Reference") (OtherBodyIndex :type Integer) (bFromSweep :type Boolean) (SweepResult :type "HitResult Structure (by ref)"))
  ;[1 1 1] UI Button Prompt
  (`self.ShowPromptToPlayer` OtherActor))

(event `self.ButtonUICollider2.OnComponentBeginOverlap`
  (params (OverlappedComponent :type "PrimitiveComponent Object Reference") (OtherActor :type "Actor Object Reference") (OtherComp :type "PrimitiveComponent Object Reference") (OtherBodyIndex :type Integer) (bFromSweep :type Boolean) (SweepResult :type "HitResult Structure (by ref)"))
  ;[1 1 1] UI Button Prompt
  (`self.ShowPromptToPlayer` OtherActor))

(event `self.ButtonUICollider.OnComponentEndOverlap`
  (params (OverlappedComponent :type "PrimitiveComponent Object Reference") (OtherActor :type "Actor Object Reference") (OtherComp :type "PrimitiveComponent Object Reference") (OtherBodyIndex :type Integer))
  ;[1 1 1] UI Button Prompt
  (`self.RemovePromptToPlayer` OtherActor))

(event `self.ButtonUICollider1.OnComponentEndOverlap`
  (params (OverlappedComponent :type "PrimitiveComponent Object Reference") (OtherActor :type "Actor Object Reference") (OtherComp :type "PrimitiveComponent Object Reference") (OtherBodyIndex :type Integer))
  ;[1 1 1] UI Button Prompt
  (`self.RemovePromptToPlayer` OtherActor))

(event `self.ButtonUICollider2.OnComponentEndOverlap`
  (params (OverlappedComponent :type "PrimitiveComponent Object Reference") (OtherActor :type "Actor Object Reference") (OtherComp :type "PrimitiveComponent Object Reference") (OtherBodyIndex :type Integer))
  ;[1 1 1] UI Button Prompt
  (`self.RemovePromptToPlayer` OtherActor))

(fn `UserConstructionScript`)