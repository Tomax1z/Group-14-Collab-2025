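; Mech arm actor that performs a grab and a damaging swipe, with the swipe mirrored for left or right use.
; Grab snaps the arm to a fixed relative position, calls MoveArm and restores that position after a delay.
; Swipe enables overlap damage and chains two timelines to yaw the shoulder out and back.
; A looping timer then runs down the cooldown, and collision stays on until it expires.
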(event `/Game/Tech/Mech/MechArmControls/BPI_ButtonToArm.ActivateGrab`
  ;[1 1 1] Right Arm Grab
  (`self.K2_SetActorRelativeLocation` (-8.0 700.0 100.0))
  (`self.ArmGrab`)
  (`KismetSystemLibrary.Delay` 3.0)
  (`self.K2_SetActorRelativeLocation` (-8.0 700.0 100.0)))

(event `ArmGrab`
  ;[1 1 1] Right Arm Grab
  (set `self.StartLocation` (`self.K2_GetActorLocation`))
  (`self.MoveArm`))

(event `/Game/Tech/Mech/MechArmControls/BPI_ButtonToArm.ActivateSwipe`
  (params (`isLeft?` :type Boolean))
  ;[0.1136 1 0.9602] Swipe
  ;;[1 1 1] If cooldown is less than or equal to 0, begin the swipe. Set the input for a left or right arm swipe according to the function input, enable collision and set cooldown to 5
  (if (<= (`self.Cooldown`) 0.0)
    (set `self.LeftArmSwipe?` `isLeft?`)
    (set `self.Cooldown` 5.0)
    (`PrimitiveComponent.SetCollisionEnabled` (`self.ArmCollision`) "QueryOnly")
    ;;[1 1 1] If Left Arm Swipe is true, rotation value is reversed and relative rotation is set
    (bind (_direction _rotation) (`Timeline|Timeline` :!via `PlayFromStart`)
      (:`Update`
        (if (`self.LeftArmSwipe?`)
          (`SceneComponent.K2_SetRelativeRotation` (`self._ShoulderMesh`) (`KismetMathLibrary.MakeRotator` 0.0 0.0 _rotation) false false)
          (else
            (`SceneComponent.K2_SetRelativeRotation` (`self._ShoulderMesh`) (`KismetMathLibrary.MakeRotator` 0.0 0.0 (* _rotation -1.0)) false false))))
      (:`Finished`
        ;;[1 1 1] Separate timeline for reversing the swipe
        (bind (_direction_2 _rotation_2) (`Timeline|Timeline_0` :!via `PlayFromStart`)
          (:`Update`
            (if (`self.LeftArmSwipe?`)
              (`SceneComponent.K2_SetRelativeRotation` (`self._ShoulderMesh`) (`KismetMathLibrary.MakeRotator` 0.0 0.0 _rotation_2) false false)
              (else
                (`SceneComponent.K2_SetRelativeRotation` (`self._ShoulderMesh`) (`KismetMathLibrary.MakeRotator` 0.0 0.0 (* _rotation_2 -1.0)) false false))))
          (:`Finished`
            ;;[1 1 1] Reduce cooldown timer by 0.1 every 0.01 seconds, when cooldown is less than or equal to 0, clear the timer and disable collision
            (bind _returnvalue (`KismetSystemLibrary.K2_SetTimerDelegate` (delegate `Reduce Cooldown`) 0.01 true))))))))

(event `Reduce Cooldown`
  ;[0.1136 1 0.9602] Swipe
  ;;[1 1 1] Reduce cooldown timer by 0.1 every 0.01 seconds, when cooldown is less than or equal to 0, clear the timer and disable collision
  (if (> (`self.Cooldown`) 0.0)
    (set `self.Cooldown` (- (`self.Cooldown`) 0.1))
    (else
      (`KismetSystemLibrary.K2_ClearAndInvalidateTimerHandle` (stale `/Game/Tech/Mech/MechArmControls/BPI_ButtonToArm.ActivateSwipe` _returnvalue))
      (`PrimitiveComponent.SetCollisionEnabled` (`self.ArmCollision`) "NoCollision"))))

(event `self.ArmCollision.OnComponentBeginOverlap`
  (params (OverlappedComponent :type "PrimitiveComponent Object Reference") (OtherActor :type "Actor Object Reference") (OtherComp :type "PrimitiveComponent Object Reference") (OtherBodyIndex :type Integer) (bFromSweep :type Boolean) (SweepResult :type "HitResult Structure (by ref)"))
  (`GameplayStatics.ApplyDamage` OtherActor 75.0))

(fn `UserConstructionScript`)