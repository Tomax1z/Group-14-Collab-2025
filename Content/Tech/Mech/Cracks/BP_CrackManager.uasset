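; BP_CrackManager scatters crack decals over surfaces around its Box component when play begins.
; It runs repeated multi-sphere traces on the Visibility channel between random points offset from the box center in the world XZ plane, bounded by horizontal and vertical values.
; Each hit spawns a small, long-lived MI_Crack decal at the impact point with a fixed rotation, and the traces leave persistent debug drawing.
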(event `self.ReceiveBeginPlay`
  (`/Game/Tech/Mech/Cracks/BPI_MechToCrack.E_CreateCrack` null))

(event `/Game/Tech/Mech/Cracks/BPI_MechToCrack.E_CreateCrack`
  (params (parent :type "Actor Object Reference"))
  (bind _verticalvalue (`self.verticalValue`))
  (bind _horizontalvalue (`self.horizontalValue`))
  (bind _returnvalue (+ (`SceneComponent.K2_GetComponentLocation` (`self.Box`)) (`KismetMathLibrary.MakeVector` (`KismetMathLibrary.RandomFloatInRange` (* _horizontalvalue -1.0) _horizontalvalue) 0.0 (`KismetMathLibrary.RandomFloatInRange` (* _verticalvalue -1.0) _verticalvalue))))
  (for _ (range 11)
    (bind _outhits (`KismetSystemLibrary.SphereTraceMulti` :`Start` _returnvalue :`End` _returnvalue :`Radius` 80.0 :`TraceChannel` "TraceTypeQuery1" :`DrawDebugType` "Persistent"))
    (for _array_element _outhits
      (`GameplayStatics.SpawnDecalAtLocation` "/Game/Tech/Materials/MI_Crack.MI_Crack" (5.0 5.0 5.0) (`.ImpactPoint` (`GameplayStatics.BreakHitResult` _array_element)) (struct :`Pitch` -40.0) 999.0))))

(fn `UserConstructionScript`)