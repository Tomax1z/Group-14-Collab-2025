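; BP_CrackSpawner is a Blueprint that reveals a crack decal with sound and particles when its ECreateCrack event fires.
; The decal is hidden on BeginPlay.
; ECreateCrack plays the crack sound at the Direction component's location, waits briefly, then shows the decal and spawns the shattered-glass effect there, using that component's negated world rotation.
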(event `self.ReceiveBeginPlay`
  (`SceneComponent.SetVisibility` (`self.Decal`) false false))

(event `/Game/Tech/Mech/Cracks/BPI_MechToCrack.E_CreateCrack`
  (params (parent :type "Actor Object Reference"))
  (bind _direction (`self.Direction`))
  (`GameplayStatics.PlaySoundAtLocation` "/Game/Tech/Mech/S_Crack.S_Crack" (`SceneComponent.K2_GetComponentLocation` (`self.Direction`)) (struct) 1.0 1.0 0.0 null null null null)
  (`KismetSystemLibrary.Delay` 0.8)
  (`|ExecutionSequence`
    (:`then_0`
      (`SceneComponent.SetVisibility` (`self.Decal`) true false))
    (:`then_1`
      (`NiagaraFunctionLibrary.SpawnSystemAtLocation` "/Game/VFX/VFX/NS_GlassShattered.NS_GlassShattered" (`SceneComponent.K2_GetComponentLocation` _direction) (`KismetMathLibrary.NegateRotator` (`SceneComponent.K2_GetComponentRotation` _direction))))))

(fn `UserConstructionScript`)