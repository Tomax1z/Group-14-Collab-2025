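; Health component that handles damage, hurt and death feedback, and item drops for its owning actor.
; On BeginPlay it copies CurrentHealth into MaxHealth and binds to the owner's OnTakeAnyDamage.
; Each hit sets CurrentHealth to Damage minus CurrentHealth, playing a hurt sound while the result is above zero.
; Otherwise a FlipFlop alternates per hit between death sound with Niagara effect, and spawning the drop and destroying the owner.
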(event `self.ReceiveBeginPlay`
  ;[1 1 1] Sets current health to max
  (set `self.maxHealth` (`self.currentHealth`))
  (add `Actor.OnTakeAnyDamage` (`self.GetOwner`) (delegate `AnyDamage`)))

(event `AnyDamage`
  (params (DamagedActor :type "Actor Object Reference") (Damage :type "Float (single-precision)") (DamageType :type "DamageType Object Reference") (InstigatedBy :type "Controller Object Reference") (DamageCauser :type "Actor Object Reference"))
  (bind _returnvalue (`self.GetOwner`))
  (bind _returnvalue_2 (`Actor.K2_GetActorLocation` _returnvalue))
  ;[1 1 1] Take Damage
  (set `self.currentHealth` (- Damage (`self.currentHealth`)))
  (if (<= (`self.currentHealth`) 0.0)
    (`/Engine/EditorBlueprintResources/StandardMacros.FlipFlop`
      (:`A`
        ;[1 1 1] Plays Death Sound and Spawns a Niagara Particle
        (`GameplayStatics.PlaySound2D` (`self.deathSound`) 1.0 1.0 0.0 null null)
        (`NiagaraFunctionLibrary.SpawnSystemAttached` (`self.deathParticle`) null "None" _returnvalue_2 (struct) "KeepRelativeOffset"))
      (:`B`
        ;[1 1 1] Spawns a pick-up and kills the owner
        (`|SpawnActorFromClass` (`self.itemDrop`) (`KismetMathLibrary.MakeTransform` _returnvalue_2) "Undefined" "MultiplyWithRoot" null null)
        (`Actor.K2_DestroyActor` _returnvalue)))
    (else
      (`GameplayStatics.PlaySound2D` (`self.hurtSound`) 1.0 1.0 0.0 null null))))