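; BP_SwipeArm is a swinging arm attack that destroys standard AI enemies it overlaps, as a placeholder for real damage.
; Swipe enables arm collision and yaws the shoulder through forward and reverse timelines, negating rotation for the right arm.
; A looping timer then drains the cooldown that gates new swipes, and disables collision once it runs out.
; ActivateSwipeRight triggers a right-arm swipe.
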(event `Swipe`
  (params (`Left Arm?` :type Boolean))
  ;[0.1136 1 0.9602] Swipe
  ;;[1 1 1] If cooldown is less than or equal to 0, begin the swipe. Set the input for a left or right arm swipe according to the function input, enable collision and set cooldown to 5
  (`KismetSystemLibrary.PrintString` "Hello")
  (if (<= (`self.Cooldown`) 0.0)
    (set `self.LeftArmSwipe?` `Left Arm?`)
    (set `self.Cooldown` 5.0)
    (`PrimitiveComponent.SetCollisionEnabled` (`self.Arm Collision`) "QueryOnly")
    ;;[1 1 1] If Left Arm Swipe is true, rotation value is reversed and relative rotation is set
    (bind (_direction _rotation) (`Timeline|Swipe Timeline` :!via `PlayFromStart`)
      (:`Update`
        (if (`self.LeftArmSwipe?`)
          (`SceneComponent.K2_SetRelativeRotation` (`self.Shoulder`) (`KismetMathLibrary.MakeRotator` 0.0 0.0 _rotation) false false)
          (else
            (`SceneComponent.K2_SetRelativeRotation` (`self.Shoulder`) (`KismetMathLibrary.MakeRotator` 0.0 0.0 (* _rotation -1.0)) false false))))
      (:`Finished`
        ;;[1 1 1] Separate timeline for reversing the swipe
        (bind (_direction_2 _rotation_2) (`Timeline|Reverse Swipe Timeline` :!via `PlayFromStart`)
          (:`Update`
            (if (`self.LeftArmSwipe?`)
              (`SceneComponent.K2_SetRelativeRotation` (`self.Shoulder`) (`KismetMathLibrary.MakeRotator` 0.0 0.0 _rotation_2) false false)
              (else
                (`SceneComponent.K2_SetRelativeRotation` (`self.Shoulder`) (`KismetMathLibrary.MakeRotator` 0.0 0.0 (* _rotation_2 -1.0)) false false))))
          (:`Finished`
            ;;[1 1 1] Reduce cooldown timer by 0.1 every 0.01 seconds, when cooldown is less than or equal to 0, clear the timer and disable collision
            (bind _returnvalue (`KismetSystemLibrary.K2_SetTimerDelegate` (delegate `Reduce Cooldown`) 0.01 true))))))))

(event `Reduce Cooldown`
  ;[0.1136 1 0.9602] Swipe
  ;;[1 1 1] Reduce cooldown timer by 0.1 every 0.01 seconds, when cooldown is less than or equal to 0, clear the timer and disable collision
  (if (> (`self.Cooldown`) 0.0)
    (set `self.Cooldown` (- (`self.Cooldown`) 0.1))
    (else
      (`KismetSystemLibrary.K2_ClearAndInvalidateTimerHandle` (stale `Swipe` _returnvalue))
      (`PrimitiveComponent.SetCollisionEnabled` (`self.Arm Collision`) "NoCollision"))))

(event `self.ReceiveBeginPlay`
  ;[1 1 1] Disable collision on start
  (`PrimitiveComponent.SetCollisionEnabled` (`self.Arm Collision`) "NoCollision"))

(event `self.Arm Collision.OnComponentBeginOverlap`
  (params (OverlappedComponent :type "PrimitiveComponent Object Reference") (OtherActor :type "Actor Object Reference") (OtherComp :type "PrimitiveComponent Object Reference") (OtherBodyIndex :type Integer) (bFromSweep :type Boolean) (SweepResult :type "HitResult Structure (by ref)"))
  ;[1 1 1] Placeholder for dealing damage until I figure out how to call the BP_AI_StandardEnemy damage function
  (cast `/Game/Tech/AI/StandardEnemy/BP_AI_StandardEnemy` OtherActor)
  (`KismetSystemLibrary.PrintString` "Enemy Destroyed")
  (`self.K2_DestroyActor` OtherActor))

(event `/Game/Tech/Mech/MechArmControls/BPI_ButtonToArm.ActivateSwipeRight`
  (`self.Swipe` false)
  (`KismetSystemLibrary.PrintString` "Diiing"))

(fn `UserConstructionScript`)