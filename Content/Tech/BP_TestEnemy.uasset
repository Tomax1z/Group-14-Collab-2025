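; BP_TestEnemy is a simple test enemy that chases the player's BP_ProtoMech and dies when damaged.
; On BeginPlay it caches the first BP_ProtoMech and BP_SpawnManager found in the level.
; Each Tick it steps a fixed distance straight toward the mech, without scaling by delta time.
; Its Damaged event prints a debug message, increments the spawn manager's EnemiesDefeated count and destroys the actor.
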(event `self.ReceiveBeginPlay`
  (bind _outactors (`GameplayStatics.GetAllActorsOfClass` "/Game/Tech/Mech/BP_ProtoMech.BP_ProtoMech_C"))
  (set `self.Mech` (`|GetArrayItem` _outactors))
  (bind _outactors_2 (`GameplayStatics.GetAllActorsOfClass` "/Game/Tech/BP_SpawnManager.BP_SpawnManager_C"))
  (set `self.Spawn Manager` (`|GetArrayItem` _outactors_2)))

(event `self.ReceiveTick`
  (params (DeltaSeconds :type "Float (single-precision)"))
  (`self.K2_AddActorWorldTransform` (`KismetMathLibrary.MakeTransform` (* (`KismetMathLibrary.Normal` (- (`self.K2_GetActorLocation` (`self.Mech`)) (`SceneComponent.K2_GetComponentLocation` (`self.DefaultSceneRoot`)))) 5.0))))

(event `Damaged`
  (bind _spawn_manager (`self.Spawn Manager`))
  (`KismetSystemLibrary.PrintString` "Hello")
  (set `/Game/Tech/BP_SpawnManager.EnemiesDefeated` (+ (`/Game/Tech/BP_SpawnManager.EnemiesDefeated` _spawn_manager) 1) _spawn_manager)
  (`self.K2_DestroyActor`))

(fn `UserConstructionScript`)