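; BP_AI_StandardEnemy is the standard AI enemy Blueprint, providing a forward melee-style attack on top of its parent class.
; AttackCommand runs a sphere trace from the actor along its forward vector out to AttackDistance, filtered by ObjectTypes.
; It applies DamageDealt to the hit actor using DamageSide as the damage type, without checking whether the trace hit.
; BeginPlay and construction only call the parent.
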(event `self.ReceiveBeginPlay`
  (`parent.ReceiveBeginPlay`))

(event `/Game/Tech/AI/BPI_TreeToAI.AttackCommand`
  (bind _returnvalue (`self.K2_GetActorLocation`))
  (bind _outhit (`KismetSystemLibrary.SphereTraceSingleForObjects` _returnvalue (+ _returnvalue (* (`self.GetActorForwardVector`) (`self.Attack distance`))) 50.0 (`self.Object Types`)))
  (`GameplayStatics.ApplyDamage` (`.HitActor` (`GameplayStatics.BreakHitResult` _outhit)) (`self.DamageDealt`) null null (`self.DamageSide`)))

(fn `UserConstructionScript`
  (`parent.UserConstructionScript`))