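; BPC_HealthComponent is an actor component that tracks health for its owner and reacts to damage.
; BeginPlay copies CurrentHealth into MaxHealth and binds AnyDamage to the owner's OnTakeAnyDamage.
; AnyDamage sets CurrentHealth to damage minus current health, then plays a hurt sound if the result is above zero.
; Death sound, Niagara effect, item drop and owner destruction exist but are unconnected, so never run.
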(event `self.ReceiveBeginPlay`
  ;[1 1 1] Sets current health to max
  (set `self.maxHealth` (`self.currentHealth`))
  (add `Actor.OnTakeAnyDamage` (`self.GetOwner`) (delegate `AnyDamage`)))

(event `AnyDamage`
  (params (DamagedActor :type "Actor Object Reference") (Damage :type "Float (single-precision)") (DamageType :type "DamageType Object Reference") (InstigatedBy :type "Controller Object Reference") (DamageCauser :type "Actor Object Reference"))
  ;[1 1 1] Take Damage
  (set `self.currentHealth` (- Damage (`self.currentHealth`)))
  (if (not (<= (`self.currentHealth`) 0.0))
    (`GameplayStatics.PlaySound2D` (`self.hurtSound`) 1.0 1.0 0.0 null null)))