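; Trigger-box enemy spawner that starts spawning standard, electric and oxygen AI enemies on its first overlap.
; The overlap caches the first BP_ProtoMech found and starts three timers, one per enemy type, whose repetition depends on a Looping variable.
; Each timer event spawns its enemy offset from the spawner and attaches it to the mech.
; All three share one SpawnCount, each clearing its own timer once that passes a fixed cap.
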(event `self.Box.OnComponentBeginOverlap`
  (params (OverlappedComponent :type "PrimitiveComponent Object Reference") (OtherActor :type "Actor Object Reference") (OtherComp :type "PrimitiveComponent Object Reference") (OtherBodyIndex :type Integer) (bFromSweep :type Boolean) (SweepResult :type "HitResult Structure (by ref)"))
  (bind _outactors (`GameplayStatics.GetAllActorsOfClass` "/Game/Tech/Mech/BP_ProtoMech.BP_ProtoMech_C"))
  (set `self.MechRef` (`|GetArrayItem` _outactors))
  (`/Engine/EditorBlueprintResources/StandardMacros.DoOnce` false
    (:`Completed`
      (bind _returnvalue (`KismetSystemLibrary.K2_SetTimerDelegate` (delegate `SpawnNormalEnemy`) 2.0 (`self.Looping`)))
      (set `self.SpawnTimer` _returnvalue)
      (bind _returnvalue_2 (`KismetSystemLibrary.K2_SetTimerDelegate` (delegate `SpawnElectricEnemy`) 2.0 (`self.Looping`)))
      (set `self.SpawnTimer2` _returnvalue_2)
      (bind _returnvalue_3 (`KismetSystemLibrary.K2_SetTimerDelegate` (delegate `SpawnOxygenEnemy`) 2.0 (`self.Looping`)))
      (set `self.SpawnTimer3` _returnvalue_3))))

(event `SpawnNormalEnemy`
  (bind _returnvalue_location (`KismetMathLibrary.BreakTransform` (`self.GetTransform`)))
  (bind _returnvalue (`|SpawnActorFromClass` "/Game/Tech/AI/StandardEnemy/BP_AI_StandardEnemy.BP_AI_StandardEnemy_C" (`KismetMathLibrary.MakeTransform` (+ _returnvalue_location (100.0 100.0 0.0))) "AlwaysSpawn" "MultiplyWithRoot" null null))
  (`self.K2_AttachToActor` _returnvalue (`self.MechRef`) "None" "KeepRelative" "KeepRelative" "KeepRelative" true)
  (bind _result (`/Engine/EditorBlueprintResources/StandardMacros.IncrementInt` (`self.SpawnCount`))
    (:`  `
      (bind _output_get (set `self.SpawnCount` _result))
      (if (> _output_get 6)
        (`KismetSystemLibrary.K2_ClearAndInvalidateTimerHandle` (`self.SpawnTimer`))))))

(event `SpawnElectricEnemy`
  (bind _returnvalue_location (`KismetMathLibrary.BreakTransform` (`self.GetTransform`)))
  (bind _returnvalue (`|SpawnActorFromClass` "/Game/Tech/AI/ElectricEnemy/BP_AI_ElectricEnemy.BP_AI_ElectricEnemy_C" (`KismetMathLibrary.MakeTransform` (+ _returnvalue_location (100.0 100.0 0.0))) "AlwaysSpawn" "MultiplyWithRoot" null null))
  (`self.K2_AttachToActor` _returnvalue (`self.MechRef`) "None" "KeepRelative" "KeepRelative" "KeepRelative" true)
  (bind _result (`/Engine/EditorBlueprintResources/StandardMacros.IncrementInt` (`self.SpawnCount`))
    (:`  `
      (bind _output_get (set `self.SpawnCount` _result))
      (if (> _output_get 6)
        (`KismetSystemLibrary.K2_ClearAndInvalidateTimerHandle` (`self.SpawnTimer2`))))))

(event `SpawnOxygenEnemy`
  (bind _returnvalue_location (`KismetMathLibrary.BreakTransform` (`self.GetTransform`)))
  (bind _returnvalue (`|SpawnActorFromClass` "/Game/Tech/AI/OxygenEnemy/BP_AI_OxygenEnemy.BP_AI_OxygenEnemy_C" (`KismetMathLibrary.MakeTransform` (+ _returnvalue_location (100.0 100.0 0.0))) "AlwaysSpawn" "MultiplyWithRoot" null null))
  (`self.K2_AttachToActor` _returnvalue (`self.MechRef`) "None" "KeepRelative" "KeepRelative" "KeepRelative" true)
  (bind _result (`/Engine/EditorBlueprintResources/StandardMacros.IncrementInt` (`self.SpawnCount`))
    (:`  `
      (bind _output_get (set `self.SpawnCount` _result))
      (if (> _output_get 6)
        (`KismetSystemLibrary.K2_ClearAndInvalidateTimerHandle` (`self.SpawnTimer3`))))))

(fn `UserConstructionScript`)