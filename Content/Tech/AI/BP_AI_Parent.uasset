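; Parent Blueprint for AI actors, providing shared behavior startup, damage handling and a basic ranged attack.
; On BeginPlay it runs BT_AI, writes its distance-from-mech value to the blackboard and unbinds all OnTakeAnyDamage events.
; AnyDamage halves incoming damage while shielded, then forwards it to the health component.
; BasicRangedAttack spawns BP_Projectile at the actor's transform, passing on its damage side and attack damage.
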(event `self.ReceiveBeginPlay`
  ;[0 0 0] Begin Play
  (`AIController.RunBehaviorTree` (`AIBlueprintHelperLibrary.GetAIController` self) "/Game/Tech/AI/Tree/BT_AI.BT_AI")
  (`BlackboardComponent.SetValueAsFloat` (`AIBlueprintHelperLibrary.GetBlackboard` null) (`self.DistanceFromMechKey`) (`self.DistanceFromMech`))
  (clear `self.OnTakeAnyDamage`))

(event `self.ReceiveAnyDamage`
  (params (Damage :type "Float (single-precision)") (DamageType :type "DamageType Object Reference") (InstigatedBy :type "Controller Object Reference") (DamageCauser :type "Actor Object Reference"))
  (set `self.DamageToTake` Damage)
  (if (`self.isShielded`)
    (set `self.DamageToTake` (* (`self.DamageToTake`) 0.5)))
  (`/Game/Tech/Mech/BPC_HealthComponent.AnyDamage` (`self.BPC_HealthComponent`) null (`self.DamageToTake`) DamageType InstigatedBy DamageCauser))

(fn `BasicRangedAttack`
  (params (Damage :type "Float (double-precision)"))
  (returns (Projectile :type "Actor Object Reference"))
  (bind _returnvalue (`|SpawnActorFromClass` "/Game/Tech/AI/BP_Projectile.BP_Projectile_C" (`self.GetTransform`) "Undefined" "MultiplyWithRoot" null self))
  (set `/Game/Tech/AI/BP_Projectile.DamageSide` (`self.DamageSide`) _returnvalue)
  (set `/Game/Tech/AI/BP_Projectile.AttackDamage` (`local.Damage`) _returnvalue)
  (return _returnvalue))

(fn `UserConstructionScript`)