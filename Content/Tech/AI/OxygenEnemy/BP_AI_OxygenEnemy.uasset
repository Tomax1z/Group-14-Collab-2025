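; Oxygen enemy AI that fires basic ranged attacks and periodically deploys a bubble shield for its damage side.
; AttackCommand counts attacks; once the threshold is reached, a coin flip decides whether to try the special.
; The special scans actors attached to the enemy's attach parent for a same-side BP_BubbleShield.
; If none exists it spawns and attaches one there instead of attacking; otherwise it resets the counter and fires normally.
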(event `/Game/Tech/AI/BPI_TreeToAI.AttackCommand`
  (if (< (`self.AttacksSinceLastSpecial`) 11)
    (`/Engine/EditorBlueprintResources/StandardMacros.IncrementInt` (`self.AttacksSinceLastSpecial`) :!label _label
      (:`  `
        (`self.BasicRangedAttack` (`self.DamageDealt`) :!label _label_2)))
    (elif (`KismetMathLibrary.RandomBool`)
      (goto _label)
      (else
        (bind _existingbubbleonside_ (`self.CheckForExistingBubbleOnSide`))
        (if _existingbubbleonside_
          (set `self.AttacksSinceLastSpecial` 0)
          (goto _label_2)
          (else
            ;[1 1 1] Spawn bubble shield
            (set `self.AttacksSinceLastSpecial` 0)
            (bind _returnvalue (`|SpawnActorFromClass` "/Game/Tech/AI/OxygenEnemy/BP_BubbleShield.BP_BubbleShield_C" (`SceneComponent.GetRelativeTransform` (`self.CapsuleComponent`)) "Undefined" "MultiplyWithRoot" null null))
            (set `/Game/Tech/AI/OxygenEnemy/BP_BubbleShield.curSide` (`self.DamageSide`) _returnvalue)
            (`self.K2_AttachToActor` _returnvalue (`self.GetAttachParentActor`) "None" "KeepRelative" "KeepRelative" "KeepRelative" true)))))))

(fn `CheckForExistingBubbleOnSide`
  (returns (`existingBubbleOnSide?` :type Boolean))
  (locals (`isThereExistingBubbleOnSide?` :type Boolean))
  (set `local.isThereExistingBubbleOnSide?` false)
  (for _array_element (`self.GetAttachedActors` (`self.GetAttachParentActor`) true false)
    (if (`KismetMathLibrary.ClassIsChildOf` (`GameplayStatics.GetObjectClass` _array_element) "/Game/Tech/AI/OxygenEnemy/BP_BubbleShield.BP_BubbleShield_C")
      (bind _asbp_bubble_shield (cast `/Game/Tech/AI/OxygenEnemy/BP_BubbleShield` _array_element))
      (if (== (`self.DamageSide`) (`/Game/Tech/AI/OxygenEnemy/BP_BubbleShield.curSide` _asbp_bubble_shield))
        (set `local.isThereExistingBubbleOnSide?` true))))
  (return (`local.isThereExistingBubbleOnSide?`)))

(fn `UserConstructionScript`
  (`parent.UserConstructionScript`))