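; Electric enemy AI character, a child Blueprint that fights at range with an electric gun attached to its hand-slot socket on BeginPlay.
; Attack commands fire the inherited basic ranged attack; after four normal shots, each attack has a coin-flip chance to become a special with separate damage and overridden projectile velocity.
; SpawnObject spawns a fixed energy cell attached to the ResourceSpawn actor.
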(event `self.ReceiveBeginPlay`
  (bind _returnvalue (`|SpawnActorFromClass` "/Game/Art/Charaters/Energy_Character/Electric_Gun/BP_Electric_Gun.BP_Electric_Gun_C" (`SceneComponent.GetSocketTransform` (`self.Mesh`) "Gun_Slot" "RTS_World") "Undefined" "MultiplyWithRoot" null null))
  (`self.K2_AttachToComponent` _returnvalue (`self.Mesh`) "Gun_Slot" "SnapToTarget" "SnapToTarget" "SnapToTarget" true)
  (`parent.ReceiveBeginPlay`))

(event `self.SpawnObject`
  (bind _returnvalue (`|SpawnActorFromClass` "/Game/Tech/Resources/BP_EnergyCellFixed.BP_EnergyCellFixed_C" (`self.GetTransform` (`self.ResourceSpawn`)) "AdjustIfPossibleButAlwaysSpawn" "MultiplyWithRoot" null null))
  (`self.K2_AttachToActor` _returnvalue (`self.ResourceSpawn`) "None" "SnapToTarget" "KeepRelative" "KeepRelative" true))

(event `/Game/Tech/AI/BPI_TreeToAI.AttackCommand`
  (if (< (`self.AttacksSinceLastSpecial`) 4)
    (`/Engine/EditorBlueprintResources/StandardMacros.IncrementInt` (`self.AttacksSinceLastSpecial`) :!label _label
      (:`  `
        (`self.BasicRangedAttack` (`self.DamageDealt`))))
    (elif (`KismetMathLibrary.RandomBool`)
      (goto _label)
      (else
        (set `self.AttacksSinceLastSpecial` 0)
        (bind _projectile (`self.BasicRangedAttack` (`self.SpecialAttackDamage`)))
        (`ProjectileMovementComponent.SetVelocityInLocalSpace` (`self.GetComponentByClass` _projectile "/Script/Engine.ProjectileMovementComponent") (1000.0 0.0 0.0)))))
  (`self.PlayAnimMontage` "/Game/Art/Charaters/Animations/Electric_Enemy/Energy_Animations/AM_Electric_Attack.AM_Electric_Attack"))

(fn `UserConstructionScript`
  (`parent.UserConstructionScript`))