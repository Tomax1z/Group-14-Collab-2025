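; BP_BaseAI is a base AI actor with a simple health system that lets it take damage and die.
; On any damage, it subtracts the amount from current health, clamped between zero and max health, and prints the result for debugging.
; When health reaches zero, the actor destroys itself.
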(event `self.ReceiveAnyDamage`
  (params (Damage :type "Float (single-precision)") (DamageType :type "DamageType Object Reference") (InstigatedBy :type "Controller Object Reference") (DamageCauser :type "Actor Object Reference"))
  ;[0.3177 0.09928 0.09928] Health System -- when damage is dealt, take from the current health. If this reaches 0, destroy the actor.
  (bind _output_get (set `self.CurrentHealth` (`KismetMathLibrary.FClamp` (- (`self.CurrentHealth`) Damage) 0.0 (`self.MaxHealth`))))
  (`KismetSystemLibrary.PrintString` (`KismetStringLibrary.Conv_DoubleToString` _output_get))
  (if (<= (`self.CurrentHealth`) 0.0)
    (`self.K2_DestroyActor`)))

(fn `UserConstructionScript`)